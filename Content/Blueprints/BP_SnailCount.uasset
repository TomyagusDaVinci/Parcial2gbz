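; BP_SnailCount is a snail counter that reveals a platform once enough snails have been counted.
; On BeginPlay it resets the count and hides the referenced Platform actor with its collision disabled.
; AddSnail increments the count and, when it exactly equals SnailMax, unhides the platform and enables its collision.
; No logic in this Blueprint calls AddSnail, and its overlap and Tick events are empty.
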(event EventBeginPlay
  (Variables|Default|SetSnails 0)
  (Collision|SetActorEnableCollision (Variables|Default|GetPlatform) false)
  (Rendering|SetActorHiddenInGame (Variables|Default|GetPlatform) true))

(event Collision|EventActorBeginOverlap
  (params (OtherActor :type Actor%20Object%20Reference)))

(event EventTick
  (params (DeltaSeconds :type Float%20%28single-precision%29)))

(fn ConstructionScript)

(fn AddSnail
  (Variables|Default|SetSnails (+ (Variables|Default|GetSnails) 1))
  (if (== (Variables|Default|GetSnails) (Variables|Default|GetSnailMax))
    (Collision|SetActorEnableCollision (Variables|Default|GetPlatform) true)
    (Rendering|SetActorHiddenInGame (Variables|Default|GetPlatform) false)))