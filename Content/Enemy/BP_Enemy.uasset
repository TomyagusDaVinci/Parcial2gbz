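; Snail enemy that senses the player and can be stunned by a Flipendo tag.
; AI perception writes the sensed third-person character to the blackboard's PJ key and clears it when sensing fails.
; StunEnemy mirrors the tag into the Stun key, recolors a dynamic material created at BeginPlay and toggles capsule physics.
; A separate Bullet function spawns BP_Bullet at a given transform.
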(event OnTargetPerceptionUpdated(AIPerception)
  (params (Actor :type Actor%20Object%20Reference) (Stimulus :type AI%20Stimulus%20Structure))
  (bind _asbp_third_person_character (Utilities|Casting|CastToBP_ThirdPersonCharacter Actor))
  (AI|Components|Blackboard|SetValueasObject (AI|GetBlackboard (Pawn|GetController)) (Variables|Default|GetPJ) (select (.bSuccessfullySensed (Utilities|Struct|BreakAIStimulus Stimulus)) _asbp_third_person_character 0)))

(event Custom|StunEnemy
  (bind _returnvalue (Actor|ActorHasTag "Flipendo"))
  (bind _snailmaterial (Variables|Default|GetSnailMaterial))
  (bind _capsulecomponent (Variables|Collision|GetCapsuleComponent))
  ;[1 1 1] Stun
  (Development|PrintString "StunCheck")
  (AI|Components|Blackboard|SetValueasBool (AI|GetBlackboard (Pawn|GetController)) (Variables|Default|GetStun) _returnvalue)
  (if _returnvalue
    (Rendering|Material|SetVectorParameterValue _snailmaterial "BaseColor" "(R=0.070588,G=0.000000,B=1.000000,A=1.000000)" :!class /Script/Engine.MaterialInstanceDynamic)
    (Rendering|Material|SetScalarParameterValue _snailmaterial "Stun" 1.0 :!class /Script/Engine.MaterialInstanceDynamic)
    (Physics|SetSimulatePhysics _capsulecomponent true)
    (else
      (Rendering|Material|SetVectorParameterValue _snailmaterial "BaseColor" "(R=0.270588,G=0.000000,B=0.011765,A=1.000000)" :!class /Script/Engine.MaterialInstanceDynamic)
      (Rendering|Material|SetScalarParameterValue (Variables|Default|GetSnailMaterial) "Stun" 0.0 :!class /Script/Engine.MaterialInstanceDynamic)
      (Physics|SetSimulatePhysics _capsulecomponent false))))

(event EventBeginPlay
  (bind _returnvalue (Rendering|Material|CreateDynamicMaterialInstance (Rendering|Material|GetMaterial (Variables|Character|GetMesh) 0) "None" "None" :!class /Script/Engine.KismetMaterialLibrary))
  (bind _output_get (Variables|Default|SetSnailMaterial _returnvalue))
  (Rendering|Material|SetMaterial (Variables|Character|GetMesh) 0 _output_get))

(event Collision|EventActorBeginOverlap
  (params (OtherActor :type Actor%20Object%20Reference)))

(event EventTick
  (params (DeltaSeconds :type Float%20%28single-precision%29)))

(fn ConstructionScript)

(fn Bullet
  (params (Class :type Actor%20Class%20Reference) (SpawnTransform :type Transform))
  (Game|SpawnActorfromClass "/Game/Blueprints/BP_Bullet.BP_Bullet_C" SpawnTransform "Undefined" "MultiplyWithRoot" 0 5e+03 0))