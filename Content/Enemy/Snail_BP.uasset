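; Snail enemy that detects the third-person player through AI Perception and reports it to its AI Blackboard.
; Perception updates set the PJ key to the player while sensed and clear it otherwise.
; BeginPlay creates a dynamic mesh material for an emissive stun flash, but that timeline-driven logic is unconnected and never runs.
; SpawnObject spawns a BP_Bullet at a given transform, ignoring its Class input.
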(event OnTargetPerceptionUpdated(AIPerception)
  (params (Actor :type Actor%20Object%20Reference) (Stimulus :type AI%20Stimulus%20Structure))
  (bind _asbp_third_person_character (Utilities|Casting|CastToBP_ThirdPersonCharacter Actor))
  (AI|Components|Blackboard|SetValueasObject (AI|GetBlackboard (Pawn|GetController)) (Variables|Default|GetPJ) (select (.bSuccessfullySensed (Utilities|Struct|BreakAIStimulus Stimulus)) _asbp_third_person_character 0)))

(event EventBeginPlay
  (bind _returnvalue (Rendering|Material|CreateDynamicMaterialInstance (Rendering|Material|GetMaterial (Variables|Character|GetMesh) 0) "None" "None" :!class /Script/Engine.KismetMaterialLibrary))
  (bind _output_get (Variables|Default|SetSnailMaterial _returnvalue))
  (Rendering|Material|SetMaterial (Variables|Character|GetMesh) 0 _output_get))

(event Collision|EventActorBeginOverlap
  (params (OtherActor :type Actor%20Object%20Reference)))

(event EventTick
  (params (DeltaSeconds :type Float%20%28single-precision%29)))

(fn ConstructionScript)

(fn SpawnObject
  (params (Class :type Actor%20Class%20Reference) (SpawnTransform :type Transform))
  (Game|SpawnActorfromClass "/Game/Blueprints/BP_Bullet.BP_Bullet_C" SpawnTransform "Undefined" "MultiplyWithRoot" 0 5e+03 0))