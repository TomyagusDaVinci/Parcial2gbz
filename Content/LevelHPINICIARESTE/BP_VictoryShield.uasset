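; BP_VictoryShield is a spinning pickup that ends the level with a win when the player character touches it.
; Tick applies a fixed local rotation each frame, so the spin speed depends on frame rate.
; Overlap with BP_ThirdPersonCharacter pauses the game, adds the WINNER widget to the player screen and shows the mouse cursor.
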(event EventTick
  (params (DeltaSeconds :type Float%20%28single-precision%29))
  (Transformation|AddActorLocalRotation "0.000000,5.000000,0.000000" false false))

(event Collision|EventActorBeginOverlap
  (params (OtherActor :type Actor%20Object%20Reference))
  (Utilities|Casting|CastToBP_ThirdPersonCharacter OtherActor)
  (Game|SetGamePaused true)
  (bind _returnvalue (UserInterface|CreateWidget "/Game/LevelHPINICIARESTE/WINNER.WINNER_C" (Game|GetPlayerController 0)))
  (UserInterface|Viewport|AddtoPlayerScreen _returnvalue)
  (Variables|/Script/Engine.PlayerController|SetbShowMouseCursor (Game|GetPlayerController 0) true))

(fn ConstructionScript)